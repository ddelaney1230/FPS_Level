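; Enemy actor that chases the player, damages them on contact and is destroyed when its health runs out.
; Tick reissues an AI move toward the player and, at zero health, tells the Manager to decrement its spawn count before destroying itself.
; Any Box overlap costs health without filtering the other actor, while Capsule overlaps damage the first-person character.
; Logic to destroy overlapping bullets is present but unconnected.
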(event `self.ReceiveTick`
  (params (DeltaSeconds :type "Float (single-precision)"))
  (`self.FollowPlayer`)
  (if (== (`self.health`) 0)
    (bind _outactors (`GameplayStatics.GetAllActorsOfClass` "/Game/Blueprints/manager.manager_C"))
    (`/Game/Blueprints/manager.decrementSpawnCount` (`|GetArrayItem` _outactors))
    (`self.K2_DestroyActor`)))

(event `FollowPlayer`
  (`|AIMoveTo` self (0.0 0.0 0.0) (`GameplayStatics.GetPlayerCharacter` 0)))

(event `self.Box.OnComponentBeginOverlap`
  (params (OverlappedComponent :type "PrimitiveComponent Object Reference") (OtherActor :type "Actor Object Reference") (OtherComp :type "PrimitiveComponent Object Reference") (OtherBodyIndex :type Integer) (bFromSweep :type Boolean) (SweepResult :type "HitResult Structure (by ref)"))
  (bind _result (`/Engine/EditorBlueprintResources/StandardMacros.DecrementInt` (`self.health`))
    (:`  `
      (set `self.health` _result))))

(event `self.Capsule.OnComponentBeginOverlap`
  (params (OverlappedComponent :type "PrimitiveComponent Object Reference") (OtherActor :type "Actor Object Reference") (OtherComp :type "PrimitiveComponent Object Reference") (OtherBodyIndex :type Integer) (bFromSweep :type Boolean) (SweepResult :type "HitResult Structure (by ref)"))
  (bind _asbp_first_person_character (cast `/Game/FirstPerson/Blueprints/BP_FirstPersonCharacter` OtherActor))
  (`/Game/FirstPerson/Blueprints/BP_FirstPersonCharacter.recieveDamage` _asbp_first_person_character))

(fn `UserConstructionScript`)