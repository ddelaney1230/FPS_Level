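; Manager Blueprint that keeps a running count of enemies in the AmountOfEnemies variable.
; Two custom events, IncrementSpawnCount and decrementSpawnCount, raise or lower the count by one and print the new value to screen.
; BeginPlay, overlap and the construction script are empty, so the count changes only when those events are called.
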(event `decrementSpawnCount`
  (bind _result (`/Engine/EditorBlueprintResources/StandardMacros.DecrementInt` (`self.amountOfEnemies`))
    (:`  `
      (set `self.amountOfEnemies` _result)
      (`KismetSystemLibrary.PrintString` (`KismetStringLibrary.Conv_IntToString` (`self.amountOfEnemies`))))))

(event `IncrementSpawnCount`
  (bind _result (`/Engine/EditorBlueprintResources/StandardMacros.IncrementInt` (`self.amountOfEnemies`))
    (:`  `
      (set `self.amountOfEnemies` _result)
      (`KismetSystemLibrary.PrintString` (`KismetStringLibrary.Conv_IntToString` (`self.amountOfEnemies`))))))

(fn `UserConstructionScript`)