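; Enemy spawner actor that periodically spawns an EnemyAI pawn at its root component's world location.
; Tick drives a five-second Delay, after which it checks the first Manager actor's AmountOfEnemies against a cap of 24.
; Below the cap it spawns the AI and calls IncrementSpawnCount on the Manager; otherwise it loops back into the Delay.
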(event `self.ReceiveTick`
  (params (DeltaSeconds :type "Float (single-precision)"))
  (`KismetSystemLibrary.Delay` 5.0 :!label _label)
  (bind _outactors (`GameplayStatics.GetAllActorsOfClass` "/Game/Blueprints/manager.manager_C"))
  (if (< (`/Game/Blueprints/manager.amountOfEnemies` (`|GetArrayItem` _outactors)) 24)
    (`AIBlueprintHelperLibrary.SpawnAIFromClass` "/Game/Blueprints/enemyAI.enemyAI_C" null (`SceneComponent.K2_GetComponentLocation` (`self.DefaultSceneRoot`)) (struct) false null)
    (bind _outactors_2 (`GameplayStatics.GetAllActorsOfClass` "/Game/Blueprints/manager.manager_C"))
    (`/Game/Blueprints/manager.IncrementSpawnCount` (`|GetArrayItem` _outactors_2))
    (else
      (goto _label))))

(fn `UserConstructionScript`)